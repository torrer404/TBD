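; Player character component that runs a four-hit one-handed sword combo from Enhanced Input, gated by CanAttack.
; SwordAttack plays the montage selected by AttackIndex, or buffers the press in SaveAttack while an attack is active.
; Each DoOnce-guarded step advances the index after a short delay.
; AttackCombo, which has no caller in this graph, either continues with the buffered hit or calls StopCombo to reset.
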(event `self.ReceiveBeginPlay`
  (bind _asplayer_character (cast `/Game/PlayerCharacter/Blueprints/PlayerCharacter` (`self.GetOwner`)))
  (set `self.Character Mesh` (`Character.Mesh` _asplayer_character)))

(event `EnhancedInput|/Game/PlayerCharacter/Inputs/Attacks/1HSword/BasicAttack/IA_Basic1HAttack`
  (params (ActionValue :type Boolean) (ElapsedSeconds :type "Float (double-precision)") (TriggeredSeconds :type "Float (double-precision)") (InputAction :type "InputAction Object Reference" :default "/Game/PlayerCharacter/Inputs/Attacks/1HSword/BasicAttack/IA_Basic1HAttack.IA_Basic1HAttack"))
  ;[1 1 1] Attack Input
  (:`Started`
    (if (`self.CanAttack?`)
      (`self.Sword Attack`))))

(event `Basic Attack 1`
  ;[1 1 1] Basic Combo 1
  (`/Engine/EditorBlueprintResources/StandardMacros.DoOnce` false :!label _label
    (:`Completed`
      (`KismetSystemLibrary.Delay` 0.1)
      (`|PlayMontage` (`self.Character Mesh`) "/Game/PlayerCharacter/Main_Character/Animations/Attacks/1HSword/BasicAttack/Combo_Attack_03_01_Seq_Montage.Combo_Attack_03_01_Seq_Montage"
        (:`then`
          (set `self.AttackIndex` 1)
          (goto _label :!via `Reset`))))))

(event `Basic Attack 2`
  ;[1 1 1] Basic Combo 2
  (`/Engine/EditorBlueprintResources/StandardMacros.DoOnce` false :!label _label_2
    (:`Completed`
      (`KismetSystemLibrary.Delay` 0.1)
      (`|PlayMontage` (`self.Character Mesh`) "/Game/PlayerCharacter/Main_Character/Animations/Attacks/1HSword/BasicAttack/Combo_Attack_03_02_Seq_Montage.Combo_Attack_03_02_Seq_Montage"
        (:`then`
          (set `self.AttackIndex` 2)
          (goto _label_2 :!via `Reset`))))))

(event `Sword Attack`
  ;[1 1 1] Sword Attack
  (if (`self.IsAttacking?`)
    (set `self.SaveAttack?` true)
    (else
      (set `self.IsAttacking?` true)
      (switch `int` (`self.AttackIndex`) :!label _label_3
        (:`0`
          (`self.Basic Attack 1`))
        (:`1`
          (`self.Basic Attack 2`))
        (:`2`
          (`self.Basic Attack 3`))
        (:`3`
          (`self.Basic Attack 4`))))))

(event `Basic Attack 3`
  ;[1 1 1] Basic Combo 3
  (`/Engine/EditorBlueprintResources/StandardMacros.DoOnce` false :!label _label_4
    (:`Completed`
      (`KismetSystemLibrary.Delay` 0.1)
      (`|PlayMontage` (`self.Character Mesh`) "/Game/PlayerCharacter/Main_Character/Animations/Attacks/1HSword/BasicAttack/Combo_Attack_03_03_Seq_Montage.Combo_Attack_03_03_Seq_Montage"
        (:`then`
          (set `self.AttackIndex` 3)
          (goto _label_4 :!via `Reset`))))))

(event `Attack Combo`
  ;[1 1 1] Combo Continue
  (if (`self.SaveAttack?`)
    (set `self.SaveAttack?` false)
    (goto _label_3)
    (else
      (`self.Stop Combo`))))

(event `Basic Attack 4`
  ;[1 1 1] Basic Combo 4
  (`/Engine/EditorBlueprintResources/StandardMacros.DoOnce` false :!label _label_5
    (:`Completed`
      (`KismetSystemLibrary.Delay` 0.1)
      (`|PlayMontage` (`self.Character Mesh`) "/Game/PlayerCharacter/Main_Character/Animations/Attacks/1HSword/BasicAttack/Combo_Attack_03_04_Seq_Montage.Combo_Attack_03_04_Seq_Montage"
        (:`then`
          (set `self.AttackIndex` 4)
          (goto _label_5 :!via `Reset`))))))

(event `Stop Combo`
  ;[1 1 1] Stop Combo
  (set `self.IsAttacking?` false)
  (set `self.AttackIndex` 0))